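; OptitrackPlayer is a player Blueprint, apparently for OptiTrack motion capture, whose BeginPlay, Tick and construction script are all empty.
; A CheckHMD function reports whether the headset's worn state is known, but nothing in this file calls it.
; Disconnected leftover nodes print PC/VR and Raquet/RigidBody labels and set a LiveLink controller's subject to None, but never run.
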(event `self.ReceiveBeginPlay`)

(fn `CheckHMD`
  (returns (HMD :type Boolean))
  (if (`|EnumEquality` (`HeadMountedDisplayFunctionLibrary.GetHMDWornState`) "Unknown")
    (return false)
    (else
      (return true))))

(fn `UserConstructionScript`)