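; Behavior tree task that picks a random patrol destination for an Enemy_Character.
; On execute it sets the enemy's walk speed to PatrolSpeed, then searches for a random reachable navigation point within Radius of the pawn.
; The result is written to the PatrolLocation blackboard key, falling back to the pawn's current location if none is found.
; The task succeeds in both cases and fails only when the pawn is not an Enemy_Character.
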(event `self.ReceiveExecuteAI`
  (params (OwnerController :type "AIController Object Reference") (ControlledPawn :type "Pawn Object Reference"))
  (bind _returnvalue (`Actor.K2_GetActorLocation` ControlledPawn))
  (bind _patrollocation (`self.PatrolLocation`))
  (bind (_randomlocation _returnvalue_2) (`NavigationSystemV1.K2_GetRandomReachablePointInRadius` _returnvalue (`self.Radius`) null null))
  (bind _asenemy_character (cast `/Game/AI/Enemy_Character` ControlledPawn)
    (:`then`
      (`/Game/AI/Enemy_Character.Update Walk Speed` _asenemy_character (`self.PatrolSpeed`))
      (if _returnvalue_2
        (`BTFunctionLibrary.SetBlackboardValueAsVector` _patrollocation _randomlocation)
        (else
          (`BTFunctionLibrary.SetBlackboardValueAsVector` _patrollocation _returnvalue)))
      (`self.FinishExecute` true))
    (:`CastFailed`
      (`self.FinishExecute` false))))